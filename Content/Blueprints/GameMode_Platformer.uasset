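; Game mode for the platformer that handles the win and lose outcomes.
; On BeginPlay it binds to enemy and player defeat events and counts the BP_Pig actors in the level.
; Each enemy defeat lowers the count; at zero it flags the player's BP_King as the winner, then restarts the game after a delay.
; Player defeat shows WBP_DeathScreen with a fade-in animation.
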(event `self.ReceiveBeginPlay`
  (add `self.OnEnemyDefeated` (delegate `OnEnemyDefeated_Event`))
  (add `self.OnPlayerDefeated` (delegate `OnPlayerDefeated_Event`))
  (bind _outactors (`GameplayStatics.GetAllActorsOfClass` "/Game/Blueprints/Characters/Pig/BP_Pig.BP_Pig_C"))
  (set `self.NumEnemeies` (`KismetArrayLibrary.Array_Length` _outactors)))

(event `OnPlayerDefeated_Event`
  (bind _returnvalue (`|CreateWidget` "/Game/UI/WBP_DeathScreen.WBP_DeathScreen_C" (`GameplayStatics.GetPlayerController` 0)))
  (`UserWidget.AddToViewport` _returnvalue 0)
  (`UserWidget.PlayAnimation` _returnvalue (`/Game/UI/WBP_DeathScreen.FadeIn` _returnvalue) 0.0 1 "Forward" 1.0 false))

(event `OnEnemyDefeated_Event`
  (bind _output_get (set `self.NumEnemeies` (- (`self.NumEnemeies`) 1)))
  (if (== _output_get 0)
    (bind _asbp_king (cast `/Game/Blueprints/Characters/King/BP_King` (`GameplayStatics.GetPlayerCharacter` 0)))
    (set `/Game/Blueprints/Characters/King/BP_King.PlayerWon` true _asbp_king)
    (`KismetSystemLibrary.RetriggerableDelay` 10.0)
    (`self.RestartGame`)))

(fn `UserConstructionScript`)